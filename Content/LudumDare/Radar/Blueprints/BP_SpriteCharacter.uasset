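; BP_SpriteCharacter is the player's cell sprite character, which collects items, shoots projectiles and loses lives to enemies.
; Every third item grows the capsule, adds a projectile and highlights the flipbook, while shooting toward the mouse cursor shrinks it again.
; Enemy overlap resets size and ammo and respawns the cell with collision disabled.
; At zero lives, game time plus bonus points is saved to the GameInstance and Intro loads.
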(event `self.ReceiveBeginPlay`
  (set `self.StartingScale` (`SceneComponent.K2_GetComponentScale` (`self.CapsuleComponent`))))

(event `self.ReceiveActorBeginOverlap`
  (params (OtherActor :type "Actor Object Reference"))
  (bind _capsulecomponent (`self.CapsuleComponent`))
  (bind _asbp_item (cast `/Game/LudumDare/Radar/Blueprints/BP_Item` OtherActor)
    (:`then`
      (`/Engine/EditorBlueprintResources/StandardMacros.IncrementInt` (`self.ChargeCount`)
        (:`  `
          (`self.K2_DestroyActor` _asbp_item)
          (`/Engine/EditorBlueprintResources/StandardMacros.IncrementInt` (`self.ItemsRetrieved`)
            (:`  `
              (set `self.ExtraScorePoints` (+ (`self.ExtraScorePoints`) (`self.PointsForGettingAnItem`)))
              (`GameplayStatics.PlaySound2D` "/Game/LudumDare/Radar/Sounds/GetItem.GetItem")
              (if (== (`self.ChargeCount`) 3)
                (`SceneComponent.SetWorldScale3D` _capsulecomponent (+ (`SceneComponent.K2_GetComponentScale` _capsulecomponent) (0.4 0.4 0.4)))
                (`/Engine/EditorBlueprintResources/StandardMacros.IncrementInt` (`self.ProjectileCount`)
                  (:`  `
                    (set `self.ChargeCount` 0)
                    (`PaperFlipbookComponent.SetFlipbook` (`self.Sprite`) "/Game/LudumDare/Radar/Sprites/Character/FB_CellHighLight.FB_CellHighLight")))))))))
    (:`CastFailed`
      (cast `/Game/LudumDare/Radar/Blueprints/BP_Enemy` OtherActor)
      (`self.HitByEnemy`))))

(fn `GetDirectionToMouse`
  (returns (DirectionToMouse :type "Vector Structure"))
  (return (- (`.Location` (`GameplayStatics.BreakHitResult` (`PlayerController.GetHitResultUnderCursorByChannel` (`GameplayStatics.GetPlayerController` 0) "TraceTypeQuery1" true))) (`self.K2_GetActorLocation`))))

(fn `HasProjectile`
  (returns (HasProjectile :type Boolean))
  (return (> (`self.ProjectileCount`) 0)))

(fn `HitByEnemy`
  (`self.RelocateInStartPoint`)
  (`SceneComponent.SetWorldScale3D` (`self.CapsuleComponent`) (`self.StartingScale`))
  (`GameplayStatics.PlaySound2D` "/Game/LudumDare/Radar/Sounds/HitByEnemy.HitByEnemy")
  (set `self.ProjectileCount` 0)
  (set `self.ChargeCount` 0)
  (set `self.Lives` (- (`self.Lives`) 1))
  (`PaperFlipbookComponent.SetFlipbook` (`self.Sprite`) "/Game/LudumDare/Radar/Sprites/Character/FB_Cell.FB_Cell")
  (if (== (`self.Lives`) 0)
    (bind _asbp_game_instace (cast `/Game/LudumDare/Radar/Blueprints/BP_GameInstace` (`GameplayStatics.GetGameInstance`)))
    (set `/Game/LudumDare/Radar/Blueprints/BP_GameInstace.LastScore` (+ (`KismetSystemLibrary.GetGameTimeInSeconds`) (`self.ExtraScorePoints`)) _asbp_game_instace)
    (`GameplayStatics.OpenLevel` "Intro")))

(fn `KilledEnemy`
  (`/Engine/EditorBlueprintResources/StandardMacros.IncrementInt` (`self.EnemiesKilled`)
    (:`  `
      (set `self.ExtraScorePoints` (+ (`self.ExtraScorePoints`) (`self.PointsForKillingAnEnemy`))))))

(fn `RelocateInStartPoint`
  (`PrimitiveComponent.SetCollisionEnabled` (`self.CapsuleComponent`) "NoCollision")
  (`self.K2_SetActorLocation` (`self.StartLocation`))
  (bind _asbp_controller (cast `/Game/LudumDare/Radar/Blueprints/BP_Controller` (`GameplayStatics.GetPlayerController` 0)))
  (`/Game/LudumDare/Radar/Blueprints/BP_Controller.StopOnRespawn` _asbp_controller))

(fn `ShootProjectile`
  (bind _capsulecomponent (`self.CapsuleComponent`))
  (if (> (`self.ProjectileCount`) 0)
    (bind _returnvalue (`|SpawnActorFromClass` "/Game/LudumDare/Radar/Blueprints/BP_Projectile.BP_Projectile_C" (`KismetMathLibrary.MakeTransform` (`KismetMathLibrary.MakeVector` (.x (.location (`self.GetTransform`))) (.y (.location (`self.GetTransform`))) 25.0) (.rotation (`self.GetTransform`))) "Undefined" "OverrideRootScale" null self))
    (`GameplayStatics.PlaySound2D` "/Game/LudumDare/Radar/Sounds/Shoot.Shoot")
    (bind _directiontomouse (`self.GetDirectionToMouse`))
    (`/Game/LudumDare/Radar/Blueprints/BP_Projectile.SetDirection` _returnvalue _directiontomouse)
    (set `self.ProjectileCount` (- (`self.ProjectileCount`) 1))
    (`SceneComponent.SetWorldScale3D` _capsulecomponent (- (`SceneComponent.K2_GetComponentScale` _capsulecomponent) (0.4 0.4 0.4)))
    (if (== (`self.ProjectileCount`) 0)
      (`PaperFlipbookComponent.SetFlipbook` (`self.Sprite`) "/Game/LudumDare/Radar/Sprites/Character/FB_Cell.FB_Cell"))))

(fn `UserConstructionScript`)
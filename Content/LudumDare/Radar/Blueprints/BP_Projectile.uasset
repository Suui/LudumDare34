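; BP_Projectile is a 2D projectile actor for the Radar game, built on a Paper sprite and a projectile movement component.
; On BeginPlay the sprite ignores its instigator while moving.
; SetDirection normalizes the given direction by clamping its length to one and sets the velocity to that direction at max speed.
; The overlap event is an empty stub, so hits trigger no scripted effect.
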(event `self.ReceiveBeginPlay`
  (`PrimitiveComponent.IgnoreActorWhenMoving` (`self.PaperSprite`) (`self.GetInstigator`) true))

(event `self.ReceiveActorBeginOverlap`
  (params (OtherActor :type "Actor Object Reference"))
  (if true
    _))

(fn `SetDirection`
  (params (Direction :type "Vector Structure"))
  (bind _projectilemovement (`self.ProjectileMovement`))
  (set `MovementComponent.Velocity` (* (`KismetMathLibrary.ClampVectorSize` Direction 1.0 1.0) (`MovementComponent.GetMaxSpeed` _projectilemovement)) _projectilemovement))

(fn `UserConstructionScript`)
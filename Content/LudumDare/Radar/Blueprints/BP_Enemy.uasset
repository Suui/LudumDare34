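; BP_Enemy is a sprite-based enemy for the Radar game that stays invisible until revealed.
; BeginPlay sets the sprite's alpha to zero.
; Reveal sets the sprite to white and calls Hide, which restarts a timeline that drives the alpha to fade it out again.
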(event `Hide`
  (bind (_direction _alpha) (`Timeline|Timeline_0` :!via `PlayFromStart`)
    (:`Update`
      (`PaperFlipbookComponent.SetSpriteColor` (`self.Sprite`) (`KismetMathLibrary.MakeColor` 1.0 1.0 1.0 _alpha)))))

(event `self.ReceiveBeginPlay`
  (`PaperFlipbookComponent.SetSpriteColor` (`self.Sprite`) (`KismetMathLibrary.MakeColor` 1.0 1.0 1.0 0.0)))

(fn `Reveal`
  (`PaperFlipbookComponent.SetSpriteColor` (`self.Sprite`) (`KismetMathLibrary.MakeColor` 1.0 1.0 1.0))
  (`self.Hide`))

(fn `UserConstructionScript`)
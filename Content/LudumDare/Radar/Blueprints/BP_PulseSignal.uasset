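; BP_PulseSignal is a radar pulse actor that reveals enemies it touches.
; Its sphere collision grows by a fixed step every tick, so the expansion speed depends on frame rate.
; Overlapping a BP_Enemy calls Reveal on it, and the pulse destroys itself after DestroyTime elapses.
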(event `self.ReceiveBeginPlay`
  (`KismetSystemLibrary.Delay` (`self.DestroyTime`))
  (`self.K2_DestroyActor`))

(event `self.ReceiveTick`
  (params (DeltaSeconds :type "Float (single-precision)"))
  (bind _spherecollision (`self.SphereCollision`))
  (`SceneComponent.SetWorldScale3D` _spherecollision (+ (`SceneComponent.K2_GetComponentScale` _spherecollision) (0.25 0.25 0.25))))

(event `self.ReceiveActorBeginOverlap`
  (params (OtherActor :type "Actor Object Reference"))
  (bind _asbp_enemy (cast `/Game/LudumDare/Radar/Blueprints/BP_Enemy` OtherActor))
  (`/Game/LudumDare/Radar/Blueprints/BP_Enemy.Reveal` _asbp_enemy))

(fn `UserConstructionScript`)
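; Player controller for a Ludum Dare game that adds the game and crosshair widgets and drives a sprite character constantly forward.
; Tick pushes the character along its forward vector unless idle, while the MoveRight axis steers yaw and releasing Shoot calls its ShootProjectile.
; StopOnRespawn halts forward movement for IdleTime, then resumes it and restores the capsule's query and physics collision.
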(event `self.ReceiveBeginPlay`
  (bind _returnvalue (`|CreateWidget` "/Game/LudumDare/Radar/Blueprints/HUD/W_Game.W_Game_C" self))
  (`UserWidget.AddToViewport` _returnvalue 0)
  (bind _returnvalue_2 (`|CreateWidget` "/Game/LudumDare/Radar/Blueprints/HUD/W_Crosshair.W_Crosshair_C" self))
  (`UserWidget.AddToViewport` _returnvalue_2 0))

(event `self.ReceiveTick`
  (params (DeltaSeconds :type "Float (single-precision)"))
  (if (not (`self.IsIdle`))
    (`self.MoveForward`)))

(event `StopOnRespawn`
  (set `self.IsIdle` true)
  (`KismetSystemLibrary.Delay` (`self.IdleTime`))
  (set `self.IsIdle` false)
  (bind _asbp_sprite_character (cast `/Game/LudumDare/Radar/Blueprints/BP_SpriteCharacter` (`GameplayStatics.GetPlayerCharacter` 0)))
  (`PrimitiveComponent.SetCollisionEnabled` (`Character.CapsuleComponent` _asbp_sprite_character) "QueryAndPhysics"))

(event `InputAxis|MoveRight`
  (params (AxisValue :type "Float (single-precision)"))
  (`self.AddYawInput` AxisValue))

(event `InputAction|Shoot`
  (params (Key :type "Key Structure" :default "AnyKey"))
  (:`Released`
    (bind _asbp_sprite_character (cast `/Game/LudumDare/Radar/Blueprints/BP_SpriteCharacter` (`GameplayStatics.GetPlayerCharacter` 0)))
    (`/Game/LudumDare/Radar/Blueprints/BP_SpriteCharacter.ShootProjectile` _asbp_sprite_character)))

(fn `MoveForward`
  (bind _returnvalue (`GameplayStatics.GetPlayerCharacter` 0))
  (`Pawn.AddMovementInput` _returnvalue (`self.GetActorForwardVector` _returnvalue) 1.0 false))

(fn `UserConstructionScript`)
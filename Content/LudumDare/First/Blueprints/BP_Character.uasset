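; BP_Character is a player character that moves forward by momentum built from repeated left and right step presses, and can jump.
; Each LeftStep or RightStep press adds SpeedModifier to Speed, with no check that the presses alternate.
; A looping timer started on BeginPlay bleeds Speed down toward zero, while Tick feeds it into forward movement input as the scale.
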(event `self.ReceiveBeginPlay`
  (`KismetSystemLibrary.K2_SetTimerDelegate` (delegate `CustomEvent_0`) 0.5 true))

(event `CustomEvent_0`
  (bind _returnvalue (- (`self.Speed`) 0.05))
  (if (< _returnvalue 0.0)
    (set `self.Speed` 0.0)
    (else
      (set `self.Speed` _returnvalue))))

(event `self.ReceiveTick`
  (params (DeltaSeconds :type "Float (single-precision)"))
  (`self.AddMovementInput` (`self.GetActorForwardVector`) (`self.Speed`)))

(event `InputAction|RightStep`
  (params (Key :type "Key Structure" :default "AnyKey"))
  ;[1 1 1] Movement
  (:`Pressed`
    (set `self.Speed` (+ (`self.SpeedModifier`) (`self.Speed`)))))

(event `InputAction|LeftStep`
  (params (Key :type "Key Structure" :default "AnyKey"))
  ;[1 1 1] Movement
  (:`Pressed`
    (set `self.Speed` (+ (`self.SpeedModifier`) (`self.Speed`)))))

(event `InputAction|Jump`
  (params (Key :type "Key Structure" :default "AnyKey"))
  ;[1 1 1] Movement
  (:`Pressed`
    (`self.Jump`)))

(fn `UserConstructionScript`)